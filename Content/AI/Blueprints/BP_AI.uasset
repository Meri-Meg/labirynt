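; BP_AI is an AI pawn that patrols a looping route of waypoint actors.
; From BeginPlay, the FollowWaypoint event uses AI MoveTo toward the current waypoint.
; On success it advances the index, wraps to the first at the end, pauses briefly and calls itself again.
; A failed move has no handling, so the patrol stops there.
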(event `self.ReceiveBeginPlay`
  (`self.Follow Waypoint`))

(event `Follow Waypoint`
  (`|AIMoveTo` self (0.0 0.0 0.0) (`|GetArrayItem` (`self.waypoints`) (`self.currentWaypoint`))
    (:`OnSuccess`
      (`/Engine/EditorBlueprintResources/StandardMacros.IncrementInt` (`self.currentWaypoint`)
        (:`  `
          (if (>= (`self.currentWaypoint`) (`KismetArrayLibrary.Array_Length` (`self.waypoints`)))
            (set `self.currentWaypoint` 0))
          (`KismetSystemLibrary.Delay` 1.0)
          (`self.Follow Waypoint`))))))

(fn `UserConstructionScript`)