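; BTTask_WaypointPatrol is a Behavior Tree task that moves a BP_AI pawn to the next waypoint in its patrol loop.
; It sets the walk speed, then runs AIMoveTo toward the actor at the pawn's current waypoint index.
; On success it prints the index, advances it with wraparound, waits briefly and finishes successfully.
; A failed cast or move never calls FinishExecute.
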(event `self.ReceiveExecuteAI`
  (params (OwnerController :type "AIController Object Reference") (ControlledPawn :type "Pawn Object Reference"))
  (bind _asbp_ai (cast `/Game/AI/Blueprints/Blueprints/BP_AI` ControlledPawn))
  (set `CharacterMovementComponent.MaxWalkSpeed` 300.0 (`Character.CharacterMovement` _asbp_ai))
  (`|AIMoveTo` ControlledPawn (0.0 0.0 0.0) (`|GetArrayItem` (`/Game/AI/Blueprints/Blueprints/BP_AI.waypoints` _asbp_ai) (`/Game/AI/Blueprints/Blueprints/BP_AI.currentWaypoint` _asbp_ai))
    (:`OnSuccess`
      (`KismetSystemLibrary.PrintString` (`KismetStringLibrary.Conv_IntToString` (`/Game/AI/Blueprints/Blueprints/BP_AI.currentWaypoint` _asbp_ai)))
      (`/Engine/EditorBlueprintResources/StandardMacros.IncrementInt` (`/Game/AI/Blueprints/Blueprints/BP_AI.currentWaypoint` _asbp_ai)
        (:`  `
          (if (>= (`/Game/AI/Blueprints/Blueprints/BP_AI.currentWaypoint` _asbp_ai) (`KismetArrayLibrary.Array_Length` (`/Game/AI/Blueprints/Blueprints/BP_AI.waypoints` _asbp_ai)))
            (set `/Game/AI/Blueprints/Blueprints/BP_AI.currentWaypoint` 0 _asbp_ai))
          (`KismetSystemLibrary.Delay` 1.0)
          (`self.FinishExecute` true))))))