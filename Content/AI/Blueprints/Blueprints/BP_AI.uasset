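; BP_AI is an AI pawn that turns its senses into blackboard values for attacking, chasing and hearing.
; Every tick it sets the attack flag according to whether the player is within close range.
; Pawn sensing raises the player-seen flag, and a retriggerable delay clears it five seconds after the last sighting.
; Successful AI perception stimuli store their location as a vector under the "canHear?" key.
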(event `self.ReceiveTick`
  (params (DeltaSeconds :type "Float (single-precision)"))
  ;[0.05017 0.15 0 0.5] Attack
  (if (<= (`self.GetDistanceTo` self (`GameplayStatics.GetPlayerCharacter` 0)) 70)
    (`BlackboardComponent.SetValueAsBool` (`AIBlueprintHelperLibrary.GetBlackboard` (`AIBlueprintHelperLibrary.GetAIController` self)) "canAttack?" true)
    (else
      (`BlackboardComponent.SetValueAsBool` (`AIBlueprintHelperLibrary.GetBlackboard` (`AIBlueprintHelperLibrary.GetAIController` self)) "canAttack?" false))))

(event `self.PawnSensing.OnSeePawn`
  (params (Pawn :type "Pawn Object Reference"))
  ;[0.15 0.002201 0 0.5] Chase
  (cast `/Game/FirstPerson/Blueprints/BP_FirstPersonCharacter` Pawn)
  (`BlackboardComponent.SetValueAsBool` (`AIBlueprintHelperLibrary.GetBlackboard` (`AIBlueprintHelperLibrary.GetAIController` self)) "hasSeenPlayer?" true)
  (`KismetSystemLibrary.RetriggerableDelay` 5.0)
  (`BlackboardComponent.SetValueAsBool` (`AIBlueprintHelperLibrary.GetBlackboard` (`AIBlueprintHelperLibrary.GetAIController` self)) "hasSeenPlayer?" false))

(event `self.AIPerception.OnTargetPerceptionUpdated`
  (params (Actor :type "Actor Object Reference") (Stimulus :type "AIStimulus Structure"))
  (bind (_age _expirationage _strength _stimuluslocation _receiverlocation _tag _bsuccessfullysensed) (break `AIStimulus` Stimulus))
  ;[0.15 0.006669 0.1213 0.5] Hearing
  (if _bsuccessfullysensed
    (`BlackboardComponent.SetValueAsVector` (`AIBlueprintHelperLibrary.GetBlackboard` null) "canHear?" _stimuluslocation)))

(fn `UserConstructionScript`)