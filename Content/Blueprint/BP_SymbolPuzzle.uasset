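; BP_SymbolPuzzle is a sequence puzzle that raises a door when three inputs arrive in the correct order.
; Trigger overlaps and the PressButton event both advance a shared Step counter, resetting it to zero on a wrong input.
; Completing either path plays its own timeline, lerping the door upward from the location cached at BeginPlay.
; Only the PressButton path prints Step for debugging.
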(event `self.Trigger1.OnComponentBeginOverlap`
  (params (OverlappedComponent :type "PrimitiveComponent Object Reference") (OtherActor :type "Actor Object Reference") (OtherComp :type "PrimitiveComponent Object Reference") (OtherBodyIndex :type Integer) (bFromSweep :type Boolean) (SweepResult :type "HitResult Structure (by ref)"))
  (if (== (`self.Step`) 0)
    (set `self.Step` 1)
    (else
      (set `self.Step` 0))))

(event `self.Trigger2.OnComponentBeginOverlap`
  (params (OverlappedComponent :type "PrimitiveComponent Object Reference") (OtherActor :type "Actor Object Reference") (OtherComp :type "PrimitiveComponent Object Reference") (OtherBodyIndex :type Integer) (bFromSweep :type Boolean) (SweepResult :type "HitResult Structure (by ref)"))
  (if (== (`self.Step`) 1)
    (set `self.Step` 2)
    (else
      (set `self.Step` 0))))

(event `self.Trigger3.OnComponentBeginOverlap`
  (params (OverlappedComponent :type "PrimitiveComponent Object Reference") (OtherActor :type "Actor Object Reference") (OtherComp :type "PrimitiveComponent Object Reference") (OtherBodyIndex :type Integer) (bFromSweep :type Boolean) (SweepResult :type "HitResult Structure (by ref)"))
  (if (== (`self.Step`) 2)
    (set `self.Step` 3)
    (bind (_direction _newtrack_0) (`Timeline|Open door`)
      (:`Update`
        (`SceneComponent.K2_SetRelativeLocation` (`self.Door`) (`KismetMathLibrary.VLerp` (`self.DoorStartLocation`) (+ (`self.DoorStartLocation`) (0.0 0.0 300.0)) _newtrack_0) false false)))
    (else
      (set `self.Step` 0))))

(event `self.ReceiveBeginPlay`
  (set `self.DoorStartLocation` (`SceneComponent.RelativeLocation` (`self.Door`))))

(event `PressButton`
  (params (ButtonID :type Integer))
  (if (and (== (`self.Step`) 0) (== ButtonID 1))
    (set `self.Step` 1)
    (`KismetSystemLibrary.PrintString` (`KismetStringLibrary.Conv_IntToString` (`self.Step`)))
    (elif (and (== (`self.Step`) 1) (== ButtonID 2))
      (set `self.Step` 2)
      (`KismetSystemLibrary.PrintString` (`KismetStringLibrary.Conv_IntToString` (`self.Step`)))
      (elif (and (== (`self.Step`) 2) (== ButtonID 3))
        (set `self.Step` 3)
        (`KismetSystemLibrary.PrintString` (`KismetStringLibrary.Conv_IntToString` (`self.Step`)))
        (bind (_direction _newtrack_0) (`Timeline|Timeline`)
          (:`Update`
            (`SceneComponent.K2_SetRelativeLocation` (`self.Door`) (`KismetMathLibrary.VLerp` (`self.DoorStartLocation`) (+ (`self.DoorStartLocation`) (0.0 0.0 300.0)) _newtrack_0) false false)))
        (else
          (set `self.Step` 0)
          (`KismetSystemLibrary.PrintString` (`KismetStringLibrary.Conv_IntToString` (`self.Step`))))))))

(fn `UserConstructionScript`)